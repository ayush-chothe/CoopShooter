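; BP_SmolEnemy is an enemy that wanders by physics force rather than by movement input.
; Every Tick it picks a new random reachable navigation point within a radius of its location and pushes MeshComp toward it with a fixed-magnitude acceleration.
; The target is re-rolled each frame without following a path, so the push direction changes constantly.
; A short-lived debug sphere marks each chosen point.
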(event `self.ReceiveTick`
  (params (DeltaSeconds :type "Float (single-precision)"))
  (bind _returnvalue (`self.K2_GetActorLocation`))
  (bind _output_get (set `self.NextPathPoint` (`NavigationSystemV1.K2_GetRandomReachablePointInRadius` _returnvalue 1000.0 null null)))
  (bind _output_get_2 (set `self.ForceDirection` (- _output_get _returnvalue)))
  (bind _output_get_3 (set `self.ForceToMove` (* (`KismetMathLibrary.Normal` _output_get_2) 2000)))
  (`PrimitiveComponent.AddForce` (`self.MeshComp`) _output_get_3 "None" true)
  (`KismetSystemLibrary.DrawDebugSphere` (`self.NextPathPoint`) 100.0 12 (struct :`R` 1.0 :`G` 0.098958 :`B` 0.143616 :`A` 1.0) 5.0 1.0))

(fn `UserConstructionScript`)
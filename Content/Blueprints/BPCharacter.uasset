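; BPCharacter is a playable character Blueprint that carries a rifle and shows an on-screen crosshair.
; On BeginPlay it spawns a BP_Rifle owned by itself, stores it as CurrentWeapon and snaps it to the mesh's WeaponSocket.
; It then creates the WBP_CrossHair widget and adds it to the viewport.
; A left mouse button press calls Fire on CurrentWeapon, leaving the shooting logic to the weapon.
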(event `self.ReceiveBeginPlay`
  (bind _returnvalue (`|SpawnActorFromClass` "/Game/Blueprints/BP_Rifle.BP_Rifle_C" (`KismetMathLibrary.MakeTransform` (0.0 0.0 0.0)) "AlwaysSpawn" "OverrideRootScale" self null))
  (set `self.Current Weapon ` _returnvalue)
  (`self.K2_AttachToComponent` _returnvalue (`self.Mesh`) "WeaponSocket" "SnapToTarget" "SnapToTarget" "SnapToTarget" true)
  (bind _returnvalue_2 (`|CreateWidget` "/Game/UI/WBP_CrossHair.WBP_CrossHair_C"))
  (`UserWidget.AddToViewport` _returnvalue_2 0))

(event `Key|LeftMouseButton`
  (params (Key :type "Key Structure"))
  (:`Pressed`
    (`SWeapon.Fire` (`self.Current Weapon `))))

(fn `UserConstructionScript`)
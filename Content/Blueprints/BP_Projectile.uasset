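; BP_Projectile is a timed explosive projectile that detonates shortly after it begins play.
; A fixed delay on BeginPlay calls Explode, which spawns an explosion particle and applies radial damage with no falloff, credited to the instigator's controller.
; It also draws a red debug sphere at the damage radius, then destroys itself.
; The graph contains no impact or movement logic.
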(event `self.ReceiveBeginPlay`
  (`KismetSystemLibrary.Delay` 1.3)
  (`self.Explode`))

(event `Explode`
  (bind _returnvalue (`self.K2_GetActorLocation`))
  (`GameplayStatics.SpawnEmitterAtLocation` "/Game/WeaponEffects/Explosion/P_Explosion.P_Explosion" _returnvalue (`self.K2_GetActorRotation`))
  (`GameplayStatics.ApplyRadialDamage` :`BaseDamage` 50.0 :`Origin` _returnvalue :`DamageRadius` (`self.Damage Radius`) :`DamageCauser` self :`InstigatedByController` (`self.GetInstigatorController`) :`bDoFullDamage` true)
  (`KismetSystemLibrary.DrawDebugSphere` _returnvalue (`self.Damage Radius`) 12 (struct :`R` 1.0 :`A` 1.0) 1.2 2.0)
  (`self.K2_DestroyActor`))

(fn `UserConstructionScript`)